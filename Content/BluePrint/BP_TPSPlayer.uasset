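; BP_TPSPlayer is a third-person shooter player Blueprint whose graph logic is entirely inactive.
; BeginPlay, Tick and the fire and sniper-aim input events have empty bodies.
; Disconnected nodes retain logic for camera-based hitscan impacts, bullet spawning, muzzle effects, sniper UI with FOV changes, movement and handgun collision disabling.
; The construction script is empty.
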(event `self.ReceiveBeginPlay`)

(event `self.ReceiveTick`
  (params (DeltaSeconds :type "Float (single-precision)")))

(event `EnhancedInput|/Game/Input/IA_Fire`
  (params (ActionValue :type Boolean) (ElapsedSeconds :type "Float (double-precision)") (TriggeredSeconds :type "Float (double-precision)") (InputAction :type "InputAction Object Reference" :default "/Game/Input/IA_Fire.IA_Fire")))

(event `EnhancedInput|/Game/Input/IA_SniperAim`
  (params (ActionValue :type Boolean) (ElapsedSeconds :type "Float (double-precision)") (TriggeredSeconds :type "Float (double-precision)") (InputAction :type "InputAction Object Reference" :default "/Game/Input/IA_SniperAim.IA_SniperAim")))

(event `EnhancedInput|/Game/Input/IA_Fire`
  (params (ActionValue :type Boolean) (ElapsedSeconds :type "Float (double-precision)") (TriggeredSeconds :type "Float (double-precision)") (InputAction :type "InputAction Object Reference" :default "/Game/Input/IA_Fire.IA_Fire")))

(fn `UserConstructionScript`)